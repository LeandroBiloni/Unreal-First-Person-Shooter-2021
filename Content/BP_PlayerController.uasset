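; BP_PlayerController is a player controller that owns the player's HUD and relays gameplay state to it.
; SetHUDonScreen creates a BP_UserWidget, stores it as HUD and adds it to the viewport.
; Custom events forward life and cooldown bar percentages, fire power-up visibility, fire shot count and stun visibility to that widget, each guarded by a validity check.
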(event EventSetStunHud
  (params (state :type ESlateVisibility%20Enum :default "Visible"))
  (bind _hud (Variables|Default|GetHUD))
  (Utilities|IsValid _hud
    (:Is%20Valid
      (Default|SetStunVisibility _hud state))))

(event EventSetHUDonScreen
  ;[1 1 1] SetHud
  (bind _returnvalue (UserInterface|CreateWidget "/Game/BP_UserWidget.BP_UserWidget_C" self))
  (bind _output_get (Variables|Default|SetHUD _returnvalue))
  (UserInterface|Viewport|AddtoViewport _output_get 0))

(event EventUpdateLifeBarHud
  (params (LifeValuePercent :type Float%20%28single-precision%29))
  (bind _hud (Variables|Default|GetHUD))
  ;[0 1 0.1291] LifeBar
  (Utilities|IsValid _hud
    (:Is%20Valid
      (Default|UpdateLifeBar _hud LifeValuePercent))))

(event EventUpdateCooldownBarHud
  (params (CooldownPercentValue :type Float%20%28single-precision%29))
  (bind _hud (Variables|Default|GetHUD))
  ;[0 0.8435 1] CooldownBar
  (Utilities|IsValid _hud
    (:Is%20Valid
      (Default|UpdateCooldownBar _hud CooldownPercentValue))))

(event EventSetActiveFirePowerUpHud
  (params (state :type ESlateVisibility%20Enum :default "Visible"))
  (bind _hud (Variables|Default|GetHUD))
  ;[1 0.5973 0] FirePowerUpState
  (Utilities|IsValid _hud
    (:Is%20Valid
      (Default|SetFirePowerUpVisibility _hud state))))

(event EventUpdateFireAmountHud
  (params (ShotsAmount :type Integer))
  (bind _hud (Variables|Default|GetHUD))
  ;[1 0.5839 0] UpdateFireShotsAmount
  (Utilities|IsValid _hud
    (:Is%20Valid
      (Default|UpdateFireShotsAmount _hud ShotsAmount))))

(fn ConstructionScript)