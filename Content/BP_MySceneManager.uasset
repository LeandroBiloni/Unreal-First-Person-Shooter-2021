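; BP_MySceneManager is a scene manager actor that drives level progression and win or lose outcomes.
; When MyCharacter overlaps it, a switch on the current level name calls the next-level load for Lvl 1 and Lvl 2, or Win for Lvl 3.
; Tick polls the player pawn's CurrentLife and calls Lose at zero or below, with no guard against repeat calls.
; The load, Win and Lose functions are defined outside this graph.
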(event EventBeginPlay)

(event Collision|EventActorBeginOverlap
  (params (OtherActor :type Actor%20Object%20Reference))
  (Utilities|Casting|CastToMyCharacter OtherActor)
  (bind _returnvalue (Game|GetCurrentLevelName true))
  (switch string _returnvalue
    (:Lvl1
      (Development|PrintString "Load Second Level")
      (Class|MySceneManager|LoadSecondLevel))
    (:Lvl2
      (Development|PrintString "Load Third Level")
      (Class|MySceneManager|LoadThirdLevel))
    (:Lvl3
      (Development|PrintString "Load Win Screen")
      (Class|MySceneManager|Win))))

(event EventTick
  (params (DeltaSeconds :type Float%20%28single-precision%29))
  (bind _asmy_character (Utilities|Casting|CastToMyCharacter (Game|Player|GetPlayerPawn 0)))
  (if (<= (Variables|/Script/Unreal_Parcial_1.MyCharacter|GetcurrentLife _asmy_character) 0.0)
    (Development|PrintString "YOU LOSE")
    (Class|MySceneManager|Lose)))

(fn ConstructionScript)