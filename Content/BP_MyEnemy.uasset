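; BP_MyEnemy is an enemy actor that reacts to the player's pawn in one of three enum-selected modes: Look at, Follow or Avoid.
; Each Tick finds the closest overlapping actor, excluding itself and the player, then runs the current mode.
; Look at yaws toward the player; Follow also moves forward at MySpeed without sweeping.
; Avoidance is an empty stub, so the tracked obstacle does not yet affect movement.
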(event EventBeginPlay)

(event Collision|EventActorBeginOverlap
  (params (OtherActor :type Actor%20Object%20Reference)))

(event EventTick
  (params (DeltaSeconds :type Float%20%28single-precision%29))
  (Variables|Default|SetClosestObstacleToMe 0)
  (for _array_element (Collision|GetOverlappingActors 0 :!class /Script/Engine.Actor)
    (CallFunction|BeginOverlap _array_element))
  (switch Utilities|FlowControl|Switch|SwitchonBP_MyEnum (Variables|Default|GetEnum)
    (:NewEnumerator0
      (CallFunction|LookTarget))
    (:NewEnumerator1
      (CallFunction|FollowTarget DeltaSeconds))
    (:NewEnumerator2
      (CallFunction|Avoidance))))

(fn ConstructionScript)

(fn LookTarget
  (bind _returnvalue (Game|GetPlayerController 0))
  (bind _returnvalue_2 (Transformation|GetActorLocation))
  (bind _returnvalue_3 (Pawn|GetControlledPawn _returnvalue))
  (bind _returnvalue_4 (Transformation|GetActorLocation _returnvalue_3))
  (bind _returnvalue_5 (- _returnvalue_4 _returnvalue_2))
  (Transformation|SetActorRotation (Math|Conversions|RotationFromXVector (Math|Vector|MakeVector (.x _returnvalue_5) (.y _returnvalue_5) 0.0))))

(fn BeginOverlap
  (params (OverlapActor :type Actor%20Object%20Reference))
  (bind _returnvalue (Transformation|GetActorLocation))
  (if (not (or (== OverlapActor self) (== OverlapActor (Pawn|GetControlledPawn (Game|GetPlayerController 0)))))
    (if (Utilities|IsValid (Variables|Default|GetClosestObstacleToMe))
      (if (< (Math|Vector|VectorLength (- (Transformation|GetActorLocation OverlapActor) _returnvalue)) (Math|Vector|VectorLength (- (Transformation|GetActorLocation (Variables|Default|GetClosestObstacleToMe)) _returnvalue)))
        (Variables|Default|SetClosestObstacleToMe OverlapActor :!label _label))
      (else
        (goto _label)))))

(fn FollowTarget
  (params (DeltaTime :type Float%20%28single-precision%29))
  (CallFunction|LookTarget)
  (Transformation|SetActorLocation (+ (Transformation|GetActorLocation) (* (* (Transformation|GetActorForwardVector) (Variables|Default|GetMySpeed)) DeltaTime)) false false))

(fn Avoidance)