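; BP_Bullet is a projectile actor that deals damage to whatever it overlaps and then destroys itself.
; A chain of casts on overlap passes Damage to TakeDamage on MyEnemy, EnemyDebuff, TurretEnemy or EnemyStunner.
; Overlap with the player pawn is checked after MyEnemy and calls DamageCharacter, which is not defined in this graph.
; Any other overlapped actor also destroys the bullet; BeginPlay, Tick and the construction script are empty.
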(event EventBeginPlay)

(event Collision|EventActorBeginOverlap
  (params (OtherActor :type Actor%20Object%20Reference))
  (bind _damage (Variables|Default|GetDamage))
  (bind _asmy_enemy (Utilities|Casting|CastToMyEnemy OtherActor)
    (:then
      (Class|MyEnemy|TakeDamage _asmy_enemy (Variables|Default|GetDamage))
      (Actor|DestroyActor))
    (:CastFailed
      (if (Collision|IsOverlappingActor (Game|Player|GetPlayerPawn 0) :!class /Script/Engine.Actor)
        (Class|Bullet|DamageCharacter)
        (Actor|DestroyActor)
        (else
          (bind _asenemy_debuff (Utilities|Casting|CastToEnemyDebuff OtherActor)
            (:then
              (Class|EnemyDebuff|TakeDamage _asenemy_debuff _damage)
              (Actor|DestroyActor))
            (:CastFailed
              (bind _asturret_enemy (Utilities|Casting|CastToTurretEnemy OtherActor)
                (:then
                  (Class|TurretEnemy|TakeDamage _asturret_enemy _damage)
                  (Actor|DestroyActor))
                (:CastFailed
                  (bind _asenemy_stunner (Utilities|Casting|CastToEnemyStunner OtherActor)
                    (:then
                      (Class|EnemyStunner|TakeDamage _asenemy_stunner (Variables|Default|GetDamage)))
                    (:CastFailed
                      _))
                  (Actor|DestroyActor))))))))))

(event EventTick
  (params (DeltaSeconds :type Float%20%28single-precision%29)))

(fn ConstructionScript)